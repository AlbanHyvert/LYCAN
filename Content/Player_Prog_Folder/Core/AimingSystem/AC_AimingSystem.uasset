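; Aim-assist component that computes an adjusted crosshair screen position and a magnetism factor.
; A 60 Hz looping timer sphere-traces from screen center and engages the pawn hit nearest center.
; Concentric screen radii select snapping to BPI_Damageable weak or base spots (hit point otherwise), bending toward the pawn, or magnetism with a centered crosshair.
; An optional debug HUD receives the radii, crosshair position and current state.
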(event Custom|ExecuteSystem
  (bind (_bwaspawnfound _pawnscreenlocation _bdoesimplementinterface _basespotscreenlocation _weakspotscreenlocation) (CallFunction|SearchforPawntoEngage))
  (bind _adjustedcrossair (CallFunction|AdjustCrossAirScreenLocation _bwaspawnfound _pawnscreenlocation _bdoesimplementinterface _basespotscreenlocation _weakspotscreenlocation))
  (Variables|Default|SetCrossAirScreenLocation _adjustedcrossair)
  (if (Variables|Default|GetbIsDebugActivated)
    (Variables|/Game/Player_Prog_Folder/Core/AimingSystem/BPH_AimingSystem_Debug.BPH_AimingSystem_Debug_C|SetMainCrossAirLocation (Variables|Default|GetDebugHUD) (Variables|Default|GetCrossAirScreenLocation))
    (Variables|/Game/Player_Prog_Folder/Core/AimingSystem/BPH_AimingSystem_Debug.BPH_AimingSystem_Debug_C|SetCurrentSystemState (Variables|Default|GetDebugHUD) (Variables|Default|GetCurrentState))))

(event EventBeginPlay
  (bind _returnvalue (Game|GetPlayerController 0))
  (Utilities|FlowControl|Sequence
    (:then_0
      (if (Variables|Default|GetbIsDebugActivated)
        (Class|PlayerController|ClientSetHUD _returnvalue "/Game/Player_Prog_Folder/Core/AimingSystem/BPH_AimingSystem_Debug.BPH_AimingSystem_Debug_C")
        (Variables|Default|SetDebugHUD (.AsBPH%20Aiming%20System%20Debug (Utilities|Casting|CastToBPH_AimingSystem_Debug (HUD|GetHUD _returnvalue))))
        (Variables|/Game/Player_Prog_Folder/Core/AimingSystem/BPH_AimingSystem_Debug.BPH_AimingSystem_Debug_C|SetHeadshotZoneRadius (Variables|Default|GetDebugHUD) (Variables|Default|GetHeadShotZoneRadius))
        (Variables|/Game/Player_Prog_Folder/Core/AimingSystem/BPH_AimingSystem_Debug.BPH_AimingSystem_Debug_C|SetBaseshotZoneRadius (Variables|Default|GetDebugHUD) (Variables|Default|GetBaseShotZoneRadius))
        (Variables|/Game/Player_Prog_Folder/Core/AimingSystem/BPH_AimingSystem_Debug.BPH_AimingSystem_Debug_C|SetBendZoneRadius (Variables|Default|GetDebugHUD) (Variables|Default|GetBendZoneRadius))
        (Variables|/Game/Player_Prog_Folder/Core/AimingSystem/BPH_AimingSystem_Debug.BPH_AimingSystem_Debug_C|SetMagneticZone (Variables|Default|GetDebugHUD) (Variables|Default|GetMagneticZoneRadius))
        (Default|Initialize (Variables|Default|GetDebugHUD))))
    (:then_1
      (Utilities|Time|SetTimerbyEvent (delegate Custom|ExecuteSystem) 0.016667 true))))

(fn SearchforPawntoEngage
  (bind _returnvalue (Game|GetPlayerController 0))
  (bind _returnvalue_2 (Viewport|GetViewportSize))
  (bind _returnvalue_3 (* _returnvalue_2 0.5))
  (bind (_worldposition _worlddirection) (Class|GameplayStatics|DeprojectScreentoWorld _returnvalue _returnvalue_3))
  ;[1 1 1] Lance plusieurs sphères depuis le centre de l'écran pour trouver tous les pawns qui sont à peu près visible à l'écran
  (bind (_outhits _returnvalue_4) (Collision|MultiSphereTraceForObjects (+ _worldposition (* _worlddirection (Variables|Default|GetSearchTraceStartOffset))) (+ _worldposition (* _worlddirection (Variables|Default|GetSearchTraceRange))) (Variables|Default|GetSearchTraceSphereRadius) (Utilities|Array|MakeArray "ObjectTypeQuery3") false (Utilities|Array|MakeArray (Game|Player|GetPlayerPawn 0)) "None" false))
  (LocalVariables|SetLHittedPawns _outhits)
  (if _returnvalue_4
    ;[1 1 1] Pour chaque pawn touché par le multi sphere trace, on stock sa distance par rapport au centre de l'écran dans un tableau.
    (for _index (range 0 (- (Utilities|Array|Length (LocalVariables|GetLHittedPawns)) 1)) ; Petite astuce, en général c'est plus\noptimisé d'utiliser un forloop plutôt\nqu'un for each loop
      (Utilities|Array|Add (LocalVariables|GetLHittedPawnsDistToCenter) (Math|Vector|Distance2D(Vector) (/ (Viewport|GetViewportSize) 2.0) (.ScreenPosition (Class|GameplayStatics|ProjectWorldtoScreen (Game|GetPlayerController 0) (.ImpactPoint (Collision|BreakHitResult (Utilities|Array|Get(acopy) (LocalVariables|GetLHittedPawns) _index))) false)))))
    ;[1 1 1] Renvoie la position à l'écran du pawn le plus proche de l'écran
    (LocalVariables|SetLEngagedPawnScreenLocation (.ScreenPosition (Class|GameplayStatics|ProjectWorldtoScreen (Game|GetPlayerController 0) (.ImpactPoint (Collision|BreakHitResult (Utilities|Array|Get(acopy) (LocalVariables|GetLHittedPawns) (.IndexOfMinValue (Math|Float|MinOfFloatArray (LocalVariables|GetLHittedPawnsDistToCenter)))))) false)))
    (LocalVariables|SetLEngagedPawn (.HitActor (Collision|BreakHitResult (Utilities|Array|Get(acopy) (LocalVariables|GetLHittedPawns) (.IndexOfMinValue (Math|Float|MinOfFloatArray (LocalVariables|GetLHittedPawnsDistToCenter)))))))
    (if (Utilities|DoesObjectImplementInterface (LocalVariables|GetLEngagedPawn) "/Game/Player_Prog_Folder/Core/Enemy/BPI_Damageable.BPI_Damageable_C")
      (bind _screenlocation (Class|BPIDamageable|GetWeakSpotScreenLocation(Message) (LocalVariables|GetLEngagedPawn)))
      (bind _screenlocation_2 (Class|BPIDamageable|GetBaseSpotScreenLocation(Message) (LocalVariables|GetLEngagedPawn)))
      (return true (LocalVariables|GetLEngagedPawnScreenLocation) true _screenlocation_2 _screenlocation)
      (else
        (return true (LocalVariables|GetLEngagedPawnScreenLocation) false "" "")))
    (else
      (return false "(X=-1.000000,Y=-1.000000)" false "" "") ; Si on a rien touché avec notre trace\non renvoie un false et une position\nà l'écran qui est négative
    )))

(fn AdjustCrossAirScreenLocation
  (params (bWasPawnFound :type Boolean) (EngagedPawnScreenLocation :type Vector%202D%20Structure) (bDoesImplementInterface :type Boolean) (BaseSpotScreenLocation :type Vector%202D%20Structure) (WeakSpotScreenLocation :type Vector%202D%20Structure))
  (LocalVariables|SetLWasPawnFound bWasPawnFound)
  (LocalVariables|SetLEngagedPawnScreenLocation EngagedPawnScreenLocation)
  (LocalVariables|SetLDoesImplementInterface bDoesImplementInterface)
  (LocalVariables|SetLBaseSpotScreenLocation BaseSpotScreenLocation)
  (LocalVariables|SetLWeakSpotScreenLocation WeakSpotScreenLocation)
  (LocalVariables|SetLViewportCenterLocation (* (Viewport|GetViewportSize) 0.5))
  (LocalVariables|SetLEngagedPawnDistToCenter (Math|Vector|Distance2D(Vector) (LocalVariables|GetLEngagedPawnScreenLocation) (LocalVariables|GetLViewportCenterLocation)))
  ;[1 1 1] Si le pawn se trouve en dehors de la zone de bend, on n'a pas besoin d'ajuster la position du crosshair
  (if (and (LocalVariables|GetLWasPawnFound) (<= (LocalVariables|GetLEngagedPawnDistToCenter) (Variables|Default|GetBendZoneRadius)))
    (if (LocalVariables|GetLDoesImplementInterface)
      (if (<= (Math|Vector|Distance2D(Vector) (LocalVariables|GetLWeakSpotScreenLocation) (LocalVariables|GetLViewportCenterLocation)) (Variables|Default|GetHeadShotZoneRadius))
        (Variables|Default|SetCurrentState "NewEnumerator5")
        (return (LocalVariables|GetLWeakSpotScreenLocation))
        (elif (<= (LocalVariables|GetLEngagedPawnDistToCenter) (Variables|Default|GetBaseShotZoneRadius))
          (Variables|Default|SetCurrentState "NewEnumerator4")
          (return (LocalVariables|GetLBaseSpotScreenLocation))
          (else
            _)))
      (else
        ;[1 1 1] Si le pawn se trouve dans la zone de base shot, on met le crosshair au même endroit que le Hit du sphere trace
        (if (<= (LocalVariables|GetLEngagedPawnDistToCenter) (Variables|Default|GetBaseShotZoneRadius))
          (Variables|Default|SetCurrentState "NewEnumerator3")
          (return (LocalVariables|GetLEngagedPawnScreenLocation))
          (else
            _))))
    ;[1 1 1] Si le pawn se trouve dans la zone de bend on ajuste la position du crosshair
    (Variables|Default|SetCurrentState "NewEnumerator2")
    (return (+ (LocalVariables|GetLViewportCenterLocation) (* (Math|Vector2D|Normalize2D (- (LocalVariables|GetLEngagedPawnScreenLocation) (LocalVariables|GetLViewportCenterLocation))) (/ (* (Variables|Default|GetBaseShotZoneRadius) (- (Variables|Default|GetBendZoneRadius) (LocalVariables|GetLEngagedPawnDistToCenter))) (- (Variables|Default|GetBendZoneRadius) (Variables|Default|GetBaseShotZoneRadius))))))
    (else
      (Variables|Default|SetCurrentState (select (<= (LocalVariables|GetLEngagedPawnDistToCenter) (Variables|Default|GetMagneticZoneRadius)) "NewEnumerator1" "NewEnumerator0"))
      (return (LocalVariables|GetLViewportCenterLocation)))))

(fn GetCrossAirLocation
  (return (Variables|Default|GetCrossAirScreenLocation)))

(fn GetMagnetismFactor
  (return (Math|Float|SelectFloat (Variables|Default|GetMagnetismFactor) 1.0 (Utilities|Enum|Equal(Enum) (Variables|Default|GetCurrentState) "NewEnumerator1"))))