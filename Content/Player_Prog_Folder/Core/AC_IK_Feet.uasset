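; Foot IK component that computes foot and pelvis offsets to fit the Character to the ground.
; Each tick it line-traces on the Camera channel below both foot bones for floor distance and normal.
; It interpolates foot offsets, pelvis offset from the larger one, and foot rotations aligned to floor normals.
; The right foot offset interpolates from the left foot's current offset, not its own.
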(event EventTick
  (params (DeltaSeconds :type Float%20%28single-precision%29))
  (Variables|Default|SetDeltaSeconds DeltaSeconds)
  ;[1 1 1] Calcule l'offset du pied gauche
  (bind (_returnvalue _impactnormal) (CallFunction|TracefromFoot (Variables|Parameters|GetLeftFootName) (Variables|Parameters|GetTraceDistBelowCapsule)))
  (Variables|Default|SetLeftFootFloorNormal _impactnormal)
  (Variables|Default|SetLeftFootOffset (Math|Interpolation|FInterpTo (Variables|Default|GetLeftFootOffset) _returnvalue (Variables|Default|GetDeltaSeconds) (Variables|Parameters|GetInterpSpeed)))
  ;[1 1 1] Calcule l'offset du pied droit
  (bind (_returnvalue_2 _impactnormal_2) (CallFunction|TracefromFoot (Variables|Parameters|GetRightFootName) (Variables|Parameters|GetTraceDistBelowCapsule)))
  (Variables|Default|SetRightFootFloorNormal _impactnormal_2)
  (Variables|Default|SetRightFootOffset (Math|Interpolation|FInterpTo (Variables|Default|GetLeftFootOffset) _returnvalue_2 (Variables|Default|GetDeltaSeconds) (Variables|Parameters|GetInterpSpeed)))
  ;[1 1 1] Le pelvis va récupérer le plus grand offset parmi les deux pieds
  (Variables|Default|SetPelvisOffset (Math|Interpolation|FInterpTo (Variables|Default|GetPelvisOffset) (Math|Float|Max(Float) (Variables|Default|GetLeftFootOffset) (Variables|Default|GetRightFootOffset)) (Variables|Default|GetDeltaSeconds) (Variables|Parameters|GetInterpSpeed)))
  (bind _rotationoffset (CallFunction|CalculateRotationOffset (Variables|Default|GetLeftFootRotation) (Variables|Default|GetLeftFootFloorNormal)))
  (Variables|Default|SetLeftFootRotation _rotationoffset)
  (bind _rotationoffset_2 (CallFunction|CalculateRotationOffset (Variables|Default|GetRightFootRotation) (Variables|Default|GetRightFootFloorNormal)))
  (Variables|Default|SetRightFootRotation _rotationoffset_2))

(fn TracefromFoot
  (params (BoneName :type Name) (TraceDistBelowCapsule :type Float%20%28single-precision%29))
  (LocalVariables|SetL_TraceDistBelowCapsule TraceDistBelowCapsule)
  (LocalVariables|SetL_BoneLocation (Transformation|GetSocketLocation (Variables|/Script/Engine.Character|GetMesh (Variables|Default|GetCharacter)) BoneName))
  (LocalVariables|SetL_TraceStartLocation (Math|Vector|MakeVector (.x (LocalVariables|GetL_BoneLocation)) (.y (LocalVariables|GetL_BoneLocation)) (.z (Transformation|GetActorLocation (Variables|Default|GetCharacter)))))
  (LocalVariables|SetL_TraceEndLocation (Math|Vector|MakeVector (.x (LocalVariables|GetL_BoneLocation)) (.y (LocalVariables|GetL_BoneLocation)) (- (.z (Transformation|GetActorLocation (Variables|Default|GetCharacter))) (+ (Components|Capsule|GetScaledCapsuleHalfHeight (Variables|/Script/Engine.Character|GetCapsuleComponent (Variables|Default|GetCharacter))) (LocalVariables|GetL_TraceDistBelowCapsule)))))
  (bind (_outhit _returnvalue) (Collision|LineTraceByChannel (LocalVariables|GetL_TraceStartLocation) (LocalVariables|GetL_TraceEndLocation) "TraceTypeQuery2" true 0 "None"))
  (return (Math|Float|SelectFloat (- (Math|Vector|VectorLength (- (LocalVariables|GetL_TraceStartLocation) (.Location (Collision|BreakHitResult _outhit)))) (Components|Capsule|GetScaledCapsuleHalfHeight (Variables|/Script/Engine.Character|GetCapsuleComponent (Variables|Default|GetCharacter)))) 0.0 _returnvalue) (.ImpactNormal (Collision|BreakHitResult _outhit))))

(fn CalculateRotationOffset
  (params (CurrentRotation :type Rotator) (FloorNormal :type Vector))
  (bind _character (Variables|Default|GetCharacter))
  (bind _returnvalue (Transformation|GetActorUpVector _character))
  (return (Math|Interpolation|RInterpTo CurrentRotation (Math|Vector|RotatorfromAxisandAngle (Math|Vector|CrossProduct _returnvalue FloorNormal) (Class|KismetMathLibrary|DegAcos (Math|Vector|DotProduct _returnvalue FloorNormal))) (Variables|Default|GetDeltaSeconds) (Variables|Parameters|GetInterpSpeed))))