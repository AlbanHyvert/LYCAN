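; BP_EnemyMaster is an enemy Blueprint, named as a master class, that reports hits from point damage.
; PointDamage switches on the hit physical material's surface type to tell Weak Spot from Base Spot.
; Weak spot hits scale damage by HeadshotMultiplier and print a red HeadShot message, while base hits print unscaled damage as a yellow BodyShot.
; The damage is only printed to screen, with no health or death logic.
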(event Game|Damage|EventPointDamage
  (params (Damage :type Float%20%28single-precision%29) (DamageType :type Damage%20Type%20Object%20Reference) (HitLocation :type Vector :default "0, 0, 0") (HitNormal :type Vector :default "0, 0, 0") (HitComponent :type Primitive%20Component%20Object%20Reference) (BoneName :type Name :default "None") (ShotFromDirection :type Vector :default "0, 0, 0") (InstigatedBy :type Controller%20Object%20Reference) (DamageCauser :type Actor%20Object%20Reference) (HitInfo :type Hit%20Result%20Structure%20%28by%20ref%29))
  (switch Utilities|FlowControl|Switch|SwitchonEPhysicalSurface (Variables|/Script/Engine.PhysicalMaterial|GetSurfaceType (.PhysMat (Collision|BreakHitResult HitInfo)))
    (:SurfaceType1
      (Development|PrintString (Utilities|String|Append "HeadShot:" (Utilities|String|ToString(Float) (* Damage (Variables|Default|GetHeadshotMultiplier)))) true true "(R=1.000000,G=0.000000,B=0.046772,A=1.000000)" 5.0))
    (:SurfaceType2
      (Development|PrintString (Utilities|String|Append "BodyShot:" (Utilities|String|ToString(Float) Damage)) true true "(R=1.000000,G=0.910421,B=0.000000,A=1.000000)" 5.0))))

(fn ConstructionScript)